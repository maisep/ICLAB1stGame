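; A city zone trigger that records which city the player is currently in.
; When an Archer or Warrior player character begins overlapping its Box, it writes the Zone value to NowCity on that character's MainPlayerController.
; Ending the overlap resets NowCity to an empty value, without checking which zone set it.
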(event `self.Box.OnComponentBeginOverlap`
  (params (OverlappedComponent :type "PrimitiveComponent Object Reference") (OtherActor :type "Actor Object Reference") (OtherComp :type "PrimitiveComponent Object Reference") (OtherBodyIndex :type Integer) (bFromSweep :type Boolean) (SweepResult :type "HitResult Structure (by ref)"))
  (bind _zone (`self.zone`))
  (bind _asbp_player_character_archer (cast `/Game/BluePrints/Character/BP_PlayerCharacter_Archer` OtherActor)
    (:`then`
      (bind _asmain_player_controller (cast `/Game/BluePrints/MainPlayerController` (`Pawn.GetController` _asbp_player_character_archer)))
      (set `/Game/BluePrints/MainPlayerController.now_city` _zone _asmain_player_controller))
    (:`CastFailed`
      (bind _asbp_player_character_warrior (cast `/Game/BluePrints/Character/BP_PlayerCharacter_Warrior` OtherActor))
      (bind _asmain_player_controller_2 (cast `/Game/BluePrints/MainPlayerController` (`Pawn.GetController` _asbp_player_character_warrior)))
      (set `/Game/BluePrints/MainPlayerController.now_city` _zone _asmain_player_controller_2))))

(event `self.Box.OnComponentEndOverlap`
  (params (OverlappedComponent :type "PrimitiveComponent Object Reference") (OtherActor :type "Actor Object Reference") (OtherComp :type "PrimitiveComponent Object Reference") (OtherBodyIndex :type Integer))
  (bind _asbp_player_character_archer (cast `/Game/BluePrints/Character/BP_PlayerCharacter_Archer` OtherActor)
    (:`then`
      (bind _asmain_player_controller (cast `/Game/BluePrints/MainPlayerController` (`Pawn.GetController` _asbp_player_character_archer)))
      (set `/Game/BluePrints/MainPlayerController.now_city` "" _asmain_player_controller))
    (:`CastFailed`
      (bind _asbp_player_character_warrior (cast `/Game/BluePrints/Character/BP_PlayerCharacter_Warrior` OtherActor))
      (bind _asmain_player_controller_2 (cast `/Game/BluePrints/MainPlayerController` (`Pawn.GetController` _asbp_player_character_warrior)))
      (set `/Game/BluePrints/MainPlayerController.now_city` "" _asmain_player_controller_2))))

(fn `UserConstructionScript`)
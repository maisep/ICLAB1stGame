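; BP_Arrow is a bow projectile that damages monsters on hit.
; Its set_arrow_direction event sets ProjectileMovement velocity from the shooter's bow socket, aiming at the AimPoint of the shooter's Minenemytarget, or along the socket's forward vector when there is no valid target.
; ArrowCollision overlaps apply fixed damage and destroy the arrow only when they touch a BP_Monster's MonsterCollision component, ignoring all other overlaps.
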(event `self.ReceiveTick`
  (params (DeltaSeconds :type "Float (single-precision)")))

(event `self.ArrowCollision.OnComponentBeginOverlap`
  (params (OverlappedComponent :type "PrimitiveComponent Object Reference") (OtherActor :type "Actor Object Reference") (OtherComp :type "PrimitiveComponent Object Reference") (OtherBodyIndex :type Integer) (bFromSweep :type Boolean) (SweepResult :type "HitResult Structure (by ref)"))
  ;[1 1 1] Apply Arrow Damage
  (bind _asbp_monster (cast `/Game/BluePrints/Monster/MonsterBP/NormalMonster/BP_Monster` OtherActor))
  (if (== (`/Game/BluePrints/Monster/MonsterBP/NormalMonster/BP_Monster.MonsterCollision` _asbp_monster) OtherComp)
    (`GameplayStatics.ApplyDamage` _asbp_monster 100.0)
    (`self.K2_DestroyActor`)))

(event `set_arrow_direction`
  (params (ShootCharacter :type "/Game/BluePrints/Character/BP_PlayerCharacter_Archer Object Reference"))
  (bind _minenemytarget (`/Game/BluePrints/Character/BP_PlayerCharacter.minenemytarget` ShootCharacter))
  (bind _projectilemovement (`self.ProjectileMovement`))
  (bind _arrowspeed (`self.ArrowSpeed`))
  ;[1 1 1] Set Arrow Direction
  (bind _output_get (set `self.BowTransform` (`SceneComponent.GetSocketTransform` (`Character.Mesh` ShootCharacter) "BowEmitterSocket" "RTS_World")))
  (`/Engine/EditorBlueprintResources/StandardMacros.IsValid` _minenemytarget
    (:`Is Valid`
      (set `MovementComponent.Velocity` (* (`KismetMathLibrary.GetForwardVector` (`KismetMathLibrary.FindLookAtRotation` (.location _output_get) (`SceneComponent.K2_GetComponentLocation` (`/Game/BluePrints/Monster/MonsterBP/NormalMonster/BP_Monster.AimPoint` _minenemytarget)))) _arrowspeed) _projectilemovement))
    (:`Is Not Valid`
      (set `MovementComponent.Velocity` (* (`KismetMathLibrary.GetForwardVector` (.rotation _output_get)) _arrowspeed) _projectilemovement))))

(fn `UserConstructionScript`)
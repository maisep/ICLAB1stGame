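; Blueprint in the modes folder that puts the main UI widget on screen and gathers data for a minimap.
; On BeginPlay it creates Ui_main and adds it to the viewport.
; Each Tick it stores the player ThirdPersonCharacter's SceneCaptureComponent2D as Minimap and the mesh's world position as Location.
; MapIcon is a stub returning a zero location and icon size.
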(event `self.ReceiveBeginPlay`
  (bind _returnvalue (`|CreateWidget` "/Game/BluePrints/UI/ui_main.ui_main_C"))
  (`UserWidget.AddToViewport` _returnvalue 0))

(event `self.ReceiveTick`
  (params (DeltaSeconds :type "Float (single-precision)"))
  (bind _returnvalue (`GameplayStatics.GetPlayerCharacter` 0))
  (bind _asthird_person_character (cast `/Game/PN_MeadowFlowers/UE4ThirdPersonTemplate/ThirdPersonBP/Blueprints/ThirdPersonCharacter` _returnvalue))
  (set `self.minimap` (`/Game/PN_MeadowFlowers/UE4ThirdPersonTemplate/ThirdPersonBP/Blueprints/ThirdPersonCharacter.SceneCaptureComponent2D` _asthird_person_character))
  (set `self.location` (`SceneComponent.K2_GetComponentLocation` (`Character.Mesh` _returnvalue))))

(fn `Map_icon`
  (returns (location :type "Vector Structure") (icon :type "Texture Object Reference") (`icon size` :type "Vector2D Structure"))
  (return (0.0 0.0 0.0) null (0.0 0.0)))

(fn `UserConstructionScript`)
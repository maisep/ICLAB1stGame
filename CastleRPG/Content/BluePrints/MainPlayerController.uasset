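; Main player controller that handles character start-up, inventory, hotkeys and UI toggling.
; BeginPlay shows start screens or spawns and possesses the character saved in main_instance, which player_ch sets before connecting to a hard-coded IP.
; GetItems sorts items by ID prefix into three slot arrays, stacking etc/usable items to 99 and treating "etc" rows as empty.
; Hotkeys use items (village-teleport scrolls, stub heal), FlipFlops toggle widgets, and debug keys add test items.
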(event `Key|SpaceBar`
  (params (Key :type "Key Structure")))

(event `Key|Zero`
  (params (Key :type "Key Structure"))
  (bind _et_items (`self.et_items`))
  (bind _returnvalue (`KismetArrayLibrary.Array_Find` (`self.eq_items`) (make `/Game/BluePrints/UI/table/slot` "etc")))
  ;[1 1 1] 테스트 부분
  (:`Pressed`
    (`|ExecutionSequence`
      (:`then_0`
        (for _index (range 9)
          (set `self.memo_mount` 1)
          (bind _output (`|GetArrayItem` (`self.test_item_et`) _index))
          (`self.Find Item` _output)
          (if (> (`self.memo_mount`) 0)
            (bind (_index_2 _check) (`self.Find Etc` _et_items))
            (if _check
              (`KismetArrayLibrary.Array_Set` _et_items _index_2 (make `/Game/BluePrints/UI/table/slot` _output (`self.memo_mount`)))
              (else
                (`KismetSystemLibrary.PrintString` "자리없.."))))))
      (:`then_2`
        (for _index_3 (range 15)
          (set `self.memo_mount` 1)
          (bind _output_2 (`|GetArrayItem` (`self.test_item_us`) _index_3))
          (`self.Find Item` _output_2)
          (if (> (`self.memo_mount`) 0)
            (`KismetArrayLibrary.Array_Set` (`self.us_item`) (`KismetArrayLibrary.Array_Find` (`self.us_item`) (make `/Game/BluePrints/UI/table/slot` "etc")) (make `/Game/BluePrints/UI/table/slot` _output_2 (`self.memo_mount`))))))
      (:`then_3`
        ;[1 1 1] 테스트
        (for _index_4 (range 27)
          (if (!= _returnvalue -1)
            (`KismetArrayLibrary.Array_Set` (`self.eq_items`) _returnvalue (make `/Game/BluePrints/UI/table/slot` (`|GetArrayItem` (`self.test_item_eq`) _index_4) 1))))))))

(event `Key|One`
  (params (Key :type "Key Structure"))
  (:`Pressed`
    (`self.Get Items` "et00001" 99)))

(event `self.ReceiveTick`
  (params (DeltaSeconds :type "Float (single-precision)"))
  (bind _returnvalue (`GameplayStatics.GetPlayerCharacter` 0))
  (bind _asmain_instance (cast `/Game/BluePrints/main_instance` (`GameplayStatics.GetGameInstance`)))
  (set `self.As Main Instance` _asmain_instance)
  (bind _asthird_person_character (cast `/Game/PN_MeadowFlowers/UE4ThirdPersonTemplate/ThirdPersonBP/Blueprints/ThirdPersonCharacter` _returnvalue))
  (set `self.minimap` (`/Game/PN_MeadowFlowers/UE4ThirdPersonTemplate/ThirdPersonBP/Blueprints/ThirdPersonCharacter.SceneCaptureComponent2D` _asthird_person_character))
  (set `self.location` (`SceneComponent.K2_GetComponentLocation` (`Character.Mesh` _returnvalue))))

(event `get_item`
  (params (ID :type String) (amount :type Integer))
  (bind _eq_items (`self.eq_items`))
  ;[1 1 1] 아이템 추가
  (switch `string` (`KismetStringLibrary.GetSubstring` ID 0 2)
    (:`Default`
      (set `self.memo_mount` amount)
      (`self.Find Item` ID)
      (if (> (`self.memo_mount`) 0)
        (bind (_index _check) (`self.Find Etc` (`self.et_items`)))
        (if _check
          (`KismetArrayLibrary.Array_Set` (`self.et_items`) _index (make `/Game/BluePrints/UI/table/slot` ID (`self.memo_mount`)))
          (else
            (`KismetSystemLibrary.PrintString` "공간부족..")))))
    (:`eq`
      (set `self.memo_mount` 1)
      (bind (_index_2 _check_2) (`self.Find Etc` _eq_items))
      (if _check_2
        (`KismetArrayLibrary.Array_Set` _eq_items _index_2 (make `/Game/BluePrints/UI/table/slot` ID 1))
        (else
          (`KismetSystemLibrary.PrintString` "자리부족"))))
    (:`us`
      (set `self.memo_mount` amount)
      (`self.Find Item` ID)
      (if (> (`self.memo_mount`) 0)
        (bind (_index_3 _check_3) (`self.Find Etc` (`self.us_item`)))
        (if _check_3
          (`KismetArrayLibrary.Array_Set` (`self.us_item`) _index_3 (make `/Game/BluePrints/UI/table/slot` ID (`self.memo_mount`)))
          (else
            (`KismetSystemLibrary.PrintString` "공간부족..")))))))

(event `self.ReceiveBeginPlay`
  (bind _asmain_instance (cast `/Game/BluePrints/main_instance` (`GameplayStatics.GetGameInstance`)))
  (if (`/Game/BluePrints/main_instance.start_game` _asmain_instance)
    (`self.chan_ch` (`/Game/BluePrints/main_instance.start_char` _asmain_instance))
    (`self.ui_main`)
    (else
      (`self.start_ui`))))

(event `quest_o/x`
  ;[1 1 1] ui
  (`/Engine/EditorBlueprintResources/StandardMacros.FlipFlop`
    (:`A`
      (bind _returnvalue (`|CreateWidget` "/Game/BluePrints/UI/quest_ui.quest_ui_C"))
      (set `self.quest_ui` _returnvalue)
      (`UserWidget.AddToViewport` _returnvalue 0))
    (:`B`
      (`Widget.RemoveFromParent` (`self.quest_ui`)))))

(event `mine_o/x`
  ;[1 1 1] ui
  (`/Engine/EditorBlueprintResources/StandardMacros.FlipFlop`
    (:`A`
      (bind _returnvalue (`|CreateWidget` "/Game/BluePrints/UI/inventory_ui.inventory_ui_C"))
      (set `self.inventory_ui` _returnvalue)
      (`UserWidget.AddToViewport` _returnvalue 0))
    (:`B`
      (`Widget.RemoveFromParent` (`self.inventory_ui`)))))

(event `player_spawn`
  (params (location :type Integer))
  ;[1 1 1] 플레이어 텔포
  (bind _returnvalue (`|CreateWidget` "/Game/BluePrints/UI/fade_effect.fade_effect_C"))
  (`UserWidget.AddToViewport` _returnvalue 0)
  (`KismetSystemLibrary.Delay` 2.0)
  (`self.K2_SetActorLocation` (`GameplayStatics.GetPlayerPawn` 0) (`|GetArrayItem` (`self.vilige`) location) false true)
  (set `self.ui_check` false))

(event `start_ui`
  (bind _returnvalue (`|CreateWidget` "/Game/BluePrints/UI/G_start/start_main.start_main_C"))
  (`UserWidget.AddToViewport` _returnvalue 0)
  (bind _returnvalue_2 (`|CreateWidget` "/Game/BluePrints/UI/G_start/start_rogo.start_rogo_C"))
  (`UserWidget.AddToViewport` _returnvalue_2 0))

(event `enforce_o/x`
  ;[1 1 1] ui
  (`/Engine/EditorBlueprintResources/StandardMacros.FlipFlop`
    (:`A`
      (bind _returnvalue (`|CreateWidget` "/Game/BluePrints/UI/G_enforce/enforce_ui.enforce_ui_C"))
      (set `self.enforce_ui` _returnvalue)
      (`UserWidget.AddToViewport` _returnvalue 0))
    (:`B`
      (`Widget.RemoveFromParent` (`self.enforce_ui`)))))

(event `player_ch`
  (params (NewParam :type "Character Class Reference"))
  (bind _as_main_instance (`self.As Main Instance`))
  (set `/Game/BluePrints/main_instance.start_game` true _as_main_instance)
  (set `/Game/BluePrints/main_instance.start_char` NewParam _as_main_instance)
  (`GameplayStatics.OpenLevel` "203.232.193.175"))

(event `equip_o/x`
  ;[1 1 1] ui
  (`/Engine/EditorBlueprintResources/StandardMacros.FlipFlop`
    (:`A`
      (bind _returnvalue (`|CreateWidget` "/Game/BluePrints/UI/equip_ui.equip_ui_C"))
      (set `self.equip_ui` _returnvalue)
      (`UserWidget.AddToViewport` _returnvalue 0))
    (:`B`
      (`Widget.RemoveFromParent` (`self.equip_ui`)))))

(event `scroll`
  (params (scroll :type "/Game/BluePrints/UI/table/slot Structure"))
  ;[1 1 1] 마을귀환주문서
  (`self. minu_item` scroll)
  (`self.player_spawn` (`KismetStringLibrary.Conv_StringToInt` (`KismetStringLibrary.GetSubstring` (`.row_name_12_E332183A4CFCFD13BD741E9F921F545F` (break `/Game/BluePrints/UI/table/slot` scroll)) 6))))

(event `minu_item`
  (params (NewParam :type "/Game/BluePrints/UI/table/slot Structure"))
  (bind _us_item (`self.us_item`))
  ;[1 1 1] 아이템 사용처리
  (for (_array_element _array_index) _us_item
    (bind (_row_name _mount) (break `/Game/BluePrints/UI/table/slot` _array_element))
    (if (`KismetStringLibrary.EqualEqual_StrStr` (`.row_name_12_E332183A4CFCFD13BD741E9F921F545F` (break `/Game/BluePrints/UI/table/slot` NewParam)) _row_name)
      (`KismetArrayLibrary.Array_Set` _us_item _array_index (make `/Game/BluePrints/UI/table/slot` _row_name (- _mount 1)))
      (break))))

(event `ui_main`
  (bind _returnvalue (`|CreateWidget` "/Game/BluePrints/UI/ui_main.ui_main_C" self))
  (`/Engine/EditorBlueprintResources/StandardMacros.IsValid` _returnvalue
    (:`Is Valid`
      (`UserWidget.AddToViewport` _returnvalue 0))))

(event `setting_o/x`
  ;[1 1 1] ui
  (`/Engine/EditorBlueprintResources/StandardMacros.FlipFlop`
    (:`A`
      (bind _returnvalue (`|CreateWidget` "/Game/BluePrints/UI/setting_ui.setting_ui_C"))
      (set `self.setting_ui` _returnvalue)
      (`UserWidget.AddToViewport` _returnvalue 0))
    (:`B`
      (`Widget.RemoveFromParent` (`self.setting_ui`)))))

(event `map_o/x`
  ;[1 1 1] ui
  (`/Engine/EditorBlueprintResources/StandardMacros.FlipFlop`
    (:`A`
      (bind _returnvalue (`|CreateWidget` "/Game/BluePrints/UI/ALL_MAP.ALL_MAP_C"))
      (set `self.map_ui` _returnvalue)
      (`UserWidget.AddToViewport` _returnvalue 0))
    (:`B`
      (`Widget.RemoveFromParent` (`self.map_ui`)))))

(event `chan_ch`
  (params (NewParam :type "Character Class Reference"))
  (bind _returnvalue (`|SpawnActorFromClass` NewParam (`KismetMathLibrary.MakeTransform` (5500.0 300.0 1000.0)) "Undefined" "OverrideRootScale" null null))
  (`self.Possess` _returnvalue))

(event `Heal`
  ;[1 1 1] 힐팩
  (`KismetSystemLibrary.PrintString` "준비중 힐"))

(event `eq_store`
  ;[1 1 1] ui
  (`/Engine/EditorBlueprintResources/StandardMacros.FlipFlop`
    (:`A`
      (bind _returnvalue (`|CreateWidget` "/Game/BluePrints/UI/G_shop/ShopHUD_equip.ShopHUD_equip_C"))
      (set `self.eq_store_ui` _returnvalue)
      (`UserWidget.AddToViewport` _returnvalue 0))
    (:`B`
      (`Widget.RemoveFromParent` (`self.eq_store_ui`)))))

(event `us_store`
  ;[1 1 1] ui
)

(event `item_use_grup`
  (params (NewParam :type "/Game/BluePrints/UI/table/slot Structure"))
  (bind _returnvalue (`KismetStringLibrary.GetSubstring` (`.row_name_12_E332183A4CFCFD13BD741E9F921F545F` (break `/Game/BluePrints/UI/table/slot` NewParam)) 0 3))
  ;[1 1 1] 단축키 실행
  (set `self.ui_check` true)
  (if (`KismetStringLibrary.EqualEqual_StrStr` _returnvalue "us0")
    (`self.Heal`)
    (elif (`KismetStringLibrary.EqualEqual_StrStr` _returnvalue "us2")
      (`self.scroll` NewParam))))

(event `ui_group`
  (if (`self.ui_check`)
    (`/Engine/EditorBlueprintResources/StandardMacros.FlipFlop`
      (:`A`
        (bind _returnvalue (`|CreateWidget` (`self.ui_list`)))
        (set `self.ui_memo` _returnvalue)
        (`UserWidget.AddToViewport` _returnvalue 0))
      (:`B`
        (`Widget.RemoveFromParent` (`self.ui_memo`))))))

(event `Key|One`
  (params (Key :type "Key Structure"))
  ;[1 1 1] 단축키 모음
  (:`Pressed`
    (if (not (`self.ui_check`))
      (`self.item_use_grup` (`|GetArrayItem` (`self.us_hotkey`) 1)))))

(event `Key|E`
  (params (Key :type "Key Structure"))
  ;[1 1 1] 단축키 모음
  (:`Pressed`
    (`self.equip_o/x`)))

(event `Key|F`
  (params (Key :type "Key Structure"))
  (:`Pressed`
    (`self.ui_group`)))

(event `Key|Two`
  (params (Key :type "Key Structure"))
  ;[1 1 1] 단축키 모음
  (:`Pressed`
    (if (not (`self.ui_check`))
      (`self.item_use_grup` (`|GetArrayItem` (`self.us_hotkey`) 2)))))

(event `Key|Q`
  (params (Key :type "Key Structure"))
  ;[1 1 1] 단축키 모음
  (:`Pressed`
    (`self.quest_o/x`)))

(event `Key|Three`
  (params (Key :type "Key Structure"))
  ;[1 1 1] 단축키 모음
  (:`Pressed`
    (if (not (`self.ui_check`))
      (`self.item_use_grup` (`|GetArrayItem` (`self.us_hotkey`) 3)))))

(event `Key|M`
  (params (Key :type "Key Structure"))
  ;[1 1 1] 단축키 모음
  (:`Pressed`
    (`self.map_o/x`)))

(event `Key|Four`
  (params (Key :type "Key Structure"))
  ;[1 1 1] 단축키 모음
  (:`Pressed`
    (if (not (`self.ui_check`))
      (`self.item_use_grup` (`|GetArrayItem` (`self.us_hotkey`) 4)))))

(event `Key|I`
  (params (Key :type "Key Structure"))
  ;[1 1 1] 단축키 모음
  (:`Pressed`
    (`self.mine_o/x`)))

(event `Key|Escape`
  (params (Key :type "Key Structure"))
  ;[1 1 1] 단축키 모음
  (:`Pressed`
    (`self.setting_o/x`)))

(event `Key|Five`
  (params (Key :type "Key Structure"))
  ;[1 1 1] 단축키 모음
  (:`Pressed`
    (if (not (`self.ui_check`))
      (`self.item_use_grup` (`|GetArrayItem` (`self.us_hotkey`) 5)))))

(event `Key|LeftShift`
  (params (Key :type "Key Structure")))

(fn `Find Etc`
  (params (NewParam :type "Array of /Game/BluePrints/UI/table/slot Structure"))
  (returns (index :type Integer) (check :type Boolean))
  (bind _returnvalue (`KismetArrayLibrary.Array_Find` NewParam (make `/Game/BluePrints/UI/table/slot` "etc")))
  (return _returnvalue (!= _returnvalue -1)))

(fn `Find Item`
  (params (ID :type String))
  (bind _returnvalue (`KismetStringLibrary.GetSubstring` ID 0 2))
  (`|ExecutionSequence`
    (:`then_0`
      (if (`KismetStringLibrary.EqualEqual_StrStr` _returnvalue "et")
        (for (_array_element _array_index) (`self.et_items`)
          (bind (_row_name _mount) (break `/Game/BluePrints/UI/table/slot` _array_element))
          (if (and (`KismetStringLibrary.EqualEqual_StrStr` ID _row_name) (< _mount 99))
            (bind _returnvalue_2 (- 99 _mount))
            (if (> (`self.memo_mount`) _returnvalue_2)
              (set `self.ha___` _returnvalue_2)
              (`KismetArrayLibrary.Array_Set` (`self.et_items`) _array_index (make `/Game/BluePrints/UI/table/slot` _row_name 99))
              (set `self.memo_mount` (- (`self.memo_mount`) (`self.ha___`)))
              (else
                (`KismetArrayLibrary.Array_Set` (`self.et_items`) _array_index (make `/Game/BluePrints/UI/table/slot` _row_name (+ _mount (`self.memo_mount`))))
                (set `self.memo_mount` 0)
                (break)))))))
    (:`then_1`
      (if (`KismetStringLibrary.EqualEqual_StrStr` _returnvalue "us")
        (for (_array_element_2 _array_index_2) (`self.us_item`)
          (bind (_row_name_2 _mount_2) (break `/Game/BluePrints/UI/table/slot` _array_element_2))
          (if (and (`KismetStringLibrary.EqualEqual_StrStr` ID _row_name_2) (< _mount_2 99))
            (bind _returnvalue_3 (- 99 _mount_2))
            (if (> (`self.memo_mount`) _returnvalue_3)
              (set `self.ha___` _returnvalue_3)
              (`KismetArrayLibrary.Array_Set` (`self.us_item`) _array_index_2 (make `/Game/BluePrints/UI/table/slot` _row_name_2 99))
              (set `self.memo_mount` (- (`self.memo_mount`) (`self.ha___`)))
              (else
                (`KismetArrayLibrary.Array_Set` (`self.us_item`) _array_index_2 (make `/Game/BluePrints/UI/table/slot` _row_name_2 (+ _mount_2 (`self.memo_mount`))))
                (set `self.memo_mount` 0)
                (break)))))))))

(fn `Get Items`
  (params (ID :type String) (amount :type Integer))
  (returns (`no space` :type Boolean))
  (bind _eq_items (`self.eq_items`))
  ;[1 1 1] 아이템 추가
  (switch `string` (`KismetStringLibrary.GetSubstring` ID 0 2)
    (:`Default`
      (set `self.memo_mount` amount)
      (`self.Find Item` ID)
      (if (> (`self.memo_mount`) 0)
        (bind (_index _check) (`self.Find Etc` (`self.et_items`)))
        (if _check
          (`KismetArrayLibrary.Array_Set` (`self.et_items`) _index (make `/Game/BluePrints/UI/table/slot` ID (`self.memo_mount`)))
          (else
            (`KismetSystemLibrary.PrintString` "공간부족..")
            (return false)))))
    (:`eq`
      (set `self.memo_mount` 1)
      (bind (_index_2 _check_2) (`self.Find Etc` _eq_items))
      (if _check_2
        (`KismetArrayLibrary.Array_Set` _eq_items _index_2 (make `/Game/BluePrints/UI/table/slot` ID 1))
        (else
          (`KismetSystemLibrary.PrintString` "자리부족")
          (return false))))
    (:`us`
      (set `self.memo_mount` amount)
      (`self.Find Item` ID)
      (if (> (`self.memo_mount`) 0)
        (bind (_index_3 _check_3) (`self.Find Etc` (`self.us_item`)))
        (if _check_3
          (`KismetArrayLibrary.Array_Set` (`self.us_item`) _index_3 (make `/Game/BluePrints/UI/table/slot` ID (`self.memo_mount`)))
          (else
            (`KismetSystemLibrary.PrintString` "공간부족..")
            (return false))))))
  (return true))

(fn `Map_icon`
  (returns (location :type "Vector Structure") (icon :type "Texture Object Reference") (`icon size` :type "Vector2D Structure"))
  (return (0.0 0.0 0.0) null (0.0 0.0)))

(fn `UserConstructionScript`)
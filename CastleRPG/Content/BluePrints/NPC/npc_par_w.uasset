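; NPC character Blueprint that wanders the navmesh around a target actor, within a radius, both supplied through the setting event.
; From BeginPlay it loops AI moves to random navigable points, picking a new one whether a move succeeds or fails.
; Each Tick, a horizontal line trace from the capsule's axis to the Sphere component acts as an obstacle feeler, stopping movement and repathing on a blocking hit.
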(event `setting`
  (params (city_dist :type "Float (single-precision)") (target1_0 :type "TargetPoint Object Reference"))
  (set `self.city_dist` city_dist)
  (set `self.target1_0` target1_0))

(event `self.ReceiveBeginPlay`
  (`self.move_npc`))

(event `move_npc`
  (bind _randomlocation (`NavigationSystemV1.K2_GetRandomLocationInNavigableRadius` (`SceneComponent.K2_GetComponentLocation` (`Actor.RootComponent` (`self.target1_0`))) (`self.city_dist`) null null))
  (set `self.Random Location` _randomlocation)
  (`|AIMoveTo` self _randomlocation null 1000.0
    (:`OnSuccess`
      _)
    (:`OnFail`
      _))
  (`NavMovementComponent.StopActiveMovement` (`self.CharacterMovement`))
  (`self.move_npc`))

(event `self.ReceiveTick`
  (params (DeltaSeconds :type "Float (single-precision)"))
  (bind _returnvalue (`SceneComponent.K2_GetComponentLocation` (`self.Sphere`)))
  (bind _outhit (`KismetSystemLibrary.LineTraceSingleForObjects` (`KismetMathLibrary.MakeVector` (.x (`SceneComponent.K2_GetComponentLocation` (`self.CapsuleComponent`))) (.y (`SceneComponent.K2_GetComponentLocation` (`self.CapsuleComponent`))) (.z _returnvalue)) _returnvalue (`|MakeArray` "ObjectTypeQuery1" "ObjectTypeQuery8" "ObjectTypeQuery3" :!type "EObjectTypeQuery Enum")))
  (if (`GameplayStatics.BreakHitResult` _outhit)
    (`NavMovementComponent.StopActiveMovement` (`self.CharacterMovement`))
    (`self.move_npc`)))

(fn `UserConstructionScript`)
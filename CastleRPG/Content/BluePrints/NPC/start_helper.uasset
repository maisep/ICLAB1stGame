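; Start helper NPC Blueprint that flags UI availability on the player's controller while an Archer or Warrior character is inside its trigger box.
; On overlap, the hi event passes this actor's UiList to the MainPlayerController and sets UiCheck to true.
; On leaving, the bye event sets UiCheck to false without clearing the list.
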(event `self.Box.OnComponentBeginOverlap`
  (params (OverlappedComponent :type "PrimitiveComponent Object Reference") (OtherActor :type "Actor Object Reference") (OtherComp :type "PrimitiveComponent Object Reference") (OtherBodyIndex :type Integer) (bFromSweep :type Boolean) (SweepResult :type "HitResult Structure (by ref)"))
  (bind _asbp_player_character_archer (cast `/Game/BluePrints/Character/BP_PlayerCharacter_Archer` OtherActor)
    (:`then`
      (`self.hi` _asbp_player_character_archer))
    (:`CastFailed`
      (bind _asbp_player_character_warrior (cast `/Game/BluePrints/Character/BP_PlayerCharacter_Warrior` OtherActor))
      (`self.hi` _asbp_player_character_warrior))))

(event `hi`
  (params (`타깃` :type "Pawn Object Reference"))
  (bind _asmain_player_controller (cast `/Game/BluePrints/MainPlayerController` (`self.GetController` `타깃`)))
  (set `/Game/BluePrints/MainPlayerController.ui_list` (`self.Ui List`) _asmain_player_controller)
  (set `/Game/BluePrints/MainPlayerController.ui_check` true _asmain_player_controller))

(event `bye`
  (params (`타깃` :type "Pawn Object Reference"))
  (bind _asmain_player_controller (cast `/Game/BluePrints/MainPlayerController` (`self.GetController` `타깃`)))
  (set `/Game/BluePrints/MainPlayerController.ui_check` false _asmain_player_controller))

(event `self.Box.OnComponentEndOverlap`
  (params (OverlappedComponent :type "PrimitiveComponent Object Reference") (OtherActor :type "Actor Object Reference") (OtherComp :type "PrimitiveComponent Object Reference") (OtherBodyIndex :type Integer))
  (bind _asbp_player_character_archer (cast `/Game/BluePrints/Character/BP_PlayerCharacter_Archer` OtherActor)
    (:`then`
      (`self.bye` _asbp_player_character_archer))
    (:`CastFailed`
      (bind _asbp_player_character_warrior (cast `/Game/BluePrints/Character/BP_PlayerCharacter_Warrior` OtherActor))
      (`self.bye` _asbp_player_character_warrior))))

(fn `UserConstructionScript`)
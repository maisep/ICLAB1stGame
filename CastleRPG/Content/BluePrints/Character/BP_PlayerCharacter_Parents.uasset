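; Player character Blueprint, apparently a parent class, providing mouse click-to-move and nearest-target tracking.
; Holding SetDestination steers straight toward the cursor hit each tick; both press and release call SimpleMoveToLocation and spawn a cursor effect.
; Attackrange overlaps maintain a list of TestPickupItem actors, which Tick scans to store the closest as Minenemytarget.
; That target is only stored here, and is not cleared when the list empties.
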(event `self.ReceiveBeginPlay`
  (set `PlayerController.bShowMouseCursor` true (`GameplayStatics.GetPlayerController` 0)))

(event `self.ReceiveTick`
  (params (DeltaSeconds :type "Float (single-precision)"))
  (bind _returnvalue (`GameplayStatics.GetPlayerController` 0))
  (bind _inrangeactors (`self.inrangeactors`))
  (`|ExecutionSequence`
    (:`then_0`
      (if (`self.Clicking`)
        (`Controller.StopMovement` _returnvalue)
        (bind _output_get (set `self.Destination` (`.Location` (`GameplayStatics.BreakHitResult` (`PlayerController.GetHitResultUnderCursorByChannel` _returnvalue "TraceTypeQuery1" true)))))
        (`self.AddMovementInput` (`KismetMathLibrary.GetDirectionUnitVector` (`self.K2_GetActorLocation`) _output_get))))
    (:`then_1`
      (if (`KismetArrayLibrary.Array_IsNotEmpty` _inrangeactors)
        (set `self.minenemydistance` 99999999.0)
        (for _array_element _inrangeactors
          (bind _returnvalue_2 (`self.GetDistanceTo` _array_element self))
          (if (< _returnvalue_2 (`self.minenemydistance`))
            (set `self.minenemydistance` _returnvalue_2)
            (set `self.minenemytarget` _array_element)))))))

(event `InputAction|SetDestination`
  (params (Key :type "Key Structure"))
  (bind _returnvalue (`GameplayStatics.GetPlayerController` 0))
  ;[1 1 1] 이동
  (:`Pressed`
    (set `self.Clicking` true)
    (`Controller.StopMovement` _returnvalue :!label _label)
    (bind _output_get (set `self.Destination` (`.Location` (`GameplayStatics.BreakHitResult` (`PlayerController.GetHitResultUnderCursorByChannel` _returnvalue "TraceTypeQuery1" true)))))
    (`AIBlueprintHelperLibrary.SimpleMoveToLocation` _returnvalue _output_get)
    (`NiagaraFunctionLibrary.SpawnSystemAtLocation` (`self.FXCursor`) _output_get))
  (:`Released`
    (set `self.Clicking` false)
    (goto _label)))

(event `self.attackrange.OnComponentBeginOverlap`
  (params (OverlappedComponent :type "PrimitiveComponent Object Reference") (OtherActor :type "Actor Object Reference") (OtherComp :type "PrimitiveComponent Object Reference") (OtherBodyIndex :type Integer) (bFromSweep :type Boolean) (SweepResult :type "HitResult Structure (by ref)"))
  (bind _astest_pickup_item (cast `/Game/BluePrints/TestPickupItem` OtherActor))
  (`KismetArrayLibrary.Array_Add` (`self.inrangeactors`) _astest_pickup_item))

(event `self.attackrange.OnComponentEndOverlap`
  (params (OverlappedComponent :type "PrimitiveComponent Object Reference") (OtherActor :type "Actor Object Reference") (OtherComp :type "PrimitiveComponent Object Reference") (OtherBodyIndex :type Integer))
  (bind _inrangeactors (`self.inrangeactors`))
  (bind _astest_pickup_item (cast `/Game/BluePrints/TestPickupItem` OtherActor))
  (`KismetArrayLibrary.Array_Remove` _inrangeactors (`KismetArrayLibrary.Array_Find` _inrangeactors _astest_pickup_item)))

(fn `UserConstructionScript`)
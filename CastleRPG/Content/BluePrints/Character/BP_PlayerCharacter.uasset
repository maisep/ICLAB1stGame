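; Player character Blueprint that handles movement, camera control and cursor toggling.
; Movement input follows control yaw on the ground plane, and a zoom axis adjusts spring arm length within clamped limits.
; An input action toggles the mouse cursor, and look input is ignored while it shows.
; Click-to-move and nearest-BP_Monster targeting logic remain disconnected, leaving the TargetRange overlap events empty.
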(event `self.ReceiveBeginPlay`)

(event `self.ReceiveTick`
  (params (DeltaSeconds :type "Float (single-precision)")))

(event `InputAxis|CameraLength`
  (params (AxisValue :type "Float (single-precision)"))
  (bind _springarm (`self.SpringArm`))
  (bind _returnvalue (+ AxisValue (`SpringArmComponent.TargetArmLength` _springarm)))
  ;[1 1 1] 카메라 거리
  (if (> _returnvalue 4000.0)
    (set `SpringArmComponent.TargetArmLength` 4000.0 _springarm)
    (elif (< _returnvalue 500.0)
      (set `SpringArmComponent.TargetArmLength` 500.0 _springarm)
      (else
        (set `SpringArmComponent.TargetArmLength` _returnvalue _springarm)))))

(event `InputAxis|Turn` :overrideparent false
  (params (AxisValue :type "Float (single-precision)"))
  ;[1 1 1] 카메라 회전
  (if (not (`PlayerController.bShowMouseCursor` (`GameplayStatics.GetPlayerController` 0)))
    (`self.AddControllerYawInput` AxisValue)))

(event `InputAxis|MoveForward` :overrideparent false
  (params (AxisValue :type "Float (single-precision)"))
  ;[1 1 1] 이동
  (`self.AddMovementInput` (`KismetMathLibrary.GetForwardVector` (`KismetMathLibrary.MakeRotator` 0.0 0.0 (.yaw (`self.GetControlRotation`)))) AxisValue))

(event `InputAxis|LookUp` :overrideparent false
  (params (AxisValue :type "Float (single-precision)"))
  ;[1 1 1] 카메라 회전
  (if (not (`PlayerController.bShowMouseCursor` (`GameplayStatics.GetPlayerController` 0)))
    (`self.AddControllerPitchInput` AxisValue)))

(event `InputAxis|MoveRight` :overrideparent false
  (params (AxisValue :type "Float (single-precision)"))
  ;[1 1 1] 이동
  (`self.AddMovementInput` (`KismetMathLibrary.GetRightVector` (`KismetMathLibrary.MakeRotator` 0.0 0.0 (.yaw (`self.GetControlRotation`)))) AxisValue))

(event `InputAction|ShowCursor`
  (params (Key :type "Key Structure"))
  (bind _returnvalue (`GameplayStatics.GetPlayerController` 0))
  ;[1 1 1] 마우스 커서(ctrl키)
  (:`Pressed`
    (if (`PlayerController.bShowMouseCursor` _returnvalue)
      (set `PlayerController.bShowMouseCursor` false _returnvalue)
      (else
        (set `PlayerController.bShowMouseCursor` true _returnvalue)))))

(event `self.TargetRange.OnComponentBeginOverlap`
  (params (OverlappedComponent :type "PrimitiveComponent Object Reference") (OtherActor :type "Actor Object Reference") (OtherComp :type "PrimitiveComponent Object Reference") (OtherBodyIndex :type Integer) (bFromSweep :type Boolean) (SweepResult :type "HitResult Structure (by ref)")))

(event `InputAction|SetDestination`
  (params (Key :type "Key Structure"))
  ;[1 1 1] 클릭이동인데 안하기로 햇음... ㅠㅠ
)

(event `self.TargetRange.OnComponentEndOverlap`
  (params (OverlappedComponent :type "PrimitiveComponent Object Reference") (OtherActor :type "Actor Object Reference") (OtherComp :type "PrimitiveComponent Object Reference") (OtherBodyIndex :type Integer)))

(fn `UserConstructionScript`)
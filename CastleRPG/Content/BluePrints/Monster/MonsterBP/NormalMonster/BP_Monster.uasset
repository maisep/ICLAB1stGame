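; BP_Monster is a base monster character that tracks nearby players, takes damage, dies and requests a respawn.
; BeginPlay caches spawn location, transform and its BP_MonsterController.
; SearchRange overlaps keep a unique TargetPlayers list and count, accepting only player capsule hits.
; Lethal damage triggers death once, disables movement and sets a short lifespan, while attack, death motion and respawn-on-destroy are delegated through Call hooks, some named for child classes.
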(event `self.ReceiveTick`
  (params (DeltaSeconds :type "Float (single-precision)")))

(event `Get Socket`
  ;[1 1 1] Unused
  (`self.Get_Child_Socket`))

(event `self.ReceiveBeginPlay`
  ;[1 1 1] Set SpawnPoint
  (set `self.InitLocation` (`self.K2_GetActorLocation`))
  (set `self.Init Transform` (`self.GetTransform`))
  (set `self.MonsterController` (cast `/Game/BluePrints/Monster/MonsterAI/BP_MonsterController` (`self.GetController`) :!pure true)))

(event `self.ReceiveDestroyed`
  ;[1 1 1] Respawn
  (`self.RespawnMonster`))

(event `self.SearchRange.OnComponentBeginOverlap`
  (params (OverlappedComponent :type "PrimitiveComponent Object Reference") (OtherActor :type "Actor Object Reference") (OtherComp :type "PrimitiveComponent Object Reference") (OtherBodyIndex :type Integer) (bFromSweep :type Boolean) (SweepResult :type "HitResult Structure (by ref)"))
  (bind _targetplayers (`self.TargetPlayers`))
  ;[1 1 1] Get Target Player
  (bind _asbp_player_character (cast `/Game/BluePrints/Character/BP_PlayerCharacter` OtherActor))
  (if (== (`Character.CapsuleComponent` _asbp_player_character) OtherComp)
    (if (== (`KismetArrayLibrary.Array_Find` _targetplayers _asbp_player_character) -1)
      (`KismetArrayLibrary.Array_Add` _targetplayers _asbp_player_character)
      (`/Engine/EditorBlueprintResources/StandardMacros.IncrementInt` (`self.TPArraySize`)))))

(event `self.SearchRange.OnComponentEndOverlap`
  (params (OverlappedComponent :type "PrimitiveComponent Object Reference") (OtherActor :type "Actor Object Reference") (OtherComp :type "PrimitiveComponent Object Reference") (OtherBodyIndex :type Integer))
  (bind _targetplayers (`self.TargetPlayers`))
  ;[1 1 1] Get Target Player
  (bind _asbp_player_character (cast `/Game/BluePrints/Character/BP_PlayerCharacter` OtherActor))
  (if (== (`Character.CapsuleComponent` _asbp_player_character) OtherComp)
    (`KismetArrayLibrary.Array_Remove` _targetplayers (`KismetArrayLibrary.Array_Find` _targetplayers _asbp_player_character))
    (`/Engine/EditorBlueprintResources/StandardMacros.DecrementInt` (`self.TPArraySize`))))

(event `Attack`
  ;[1 1 1] Attack Motion
  (`self.Attack_Child`))

(event `self.ReceiveAnyDamage`
  (params (Damage :type "Float (single-precision)") (DamageType :type "DamageType Object Reference") (InstigatedBy :type "Controller Object Reference") (DamageCauser :type "Actor Object Reference"))
  ;[1 1 1] AnyDamage
  (bind _output_get (set `self.HP` (- (`self.HP`) Damage)))
  (if (<= _output_get 0.0)
    (`/Engine/EditorBlueprintResources/StandardMacros.DoOnce` false
      (:`Completed`
        (`self.Dead`)
        (`self.SetLifeSpan` 3.0)
        (`CharacterMovementComponent.DisableMovement` (`self.CharacterMovement`))))))

(event `Dead`
  ;[1 1 1] AnyDamage
  (`self.Dead_Motion `))

(fn `UserConstructionScript`)
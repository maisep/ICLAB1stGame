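; Poison scorpion monster Blueprint that binds parent hooks for attack, death and reward, and sets its monster code and drop table.
; Attacks pass through server and multicast events to play a montage, while a separate Damage event applies fixed damage to the first target.
; Death plays the dying animation and binds respawn, which spawns a fresh copy at the initial transform.
; Rewards use DoN-gated, cascading random rolls to grant the player an item.
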(event `C_Get_Socket`
  ;[1 1 1] Unused
  (set `self.EyeLocation` (`SceneComponent.GetSocketLocation` (`self.Mesh`) "Eyesight")))

(event `self.ReceiveBeginPlay`
  (`parent.ReceiveBeginPlay`)
  (add `self.Attack_Child` (delegate `C_Attack`))
  (add `self.Dead_Motion ` (delegate `Death`))
  (add `self.Reward` (delegate `give reward`)))

(event `C_Attack`
  ;[1 1 1] Monster's Attack
  (`self.Attack_Server` self))

(event `Death`
  ;[1 1 1] Death Animation
  (`SkeletalMeshComponent.PlayAnimation` (`self.Mesh`) "/Game/Monster/Poison_Scorpion/Anim/poison_scorpion_dying.poison_scorpion_dying" false)
  (add `self.RespawnMonster` (delegate `Respawn`)))

(event `Attack_Server`
  (params (Monster :type "/Game/BluePrints/Monster/MonsterBP/NormalMonster/BP_PoisonScorpion Object Reference"))
  ;[1 1 1] Monster's Attack
  (`self.Attack_MC` Monster))

(event `give reward` :!signature `self.Reward`
  (params (PlayerController :type "/Game/BluePrints/MainPlayerController Object Reference"))
  (bind _droptable (`self.DropTable`))
  (bind _output (`|GetArrayItem` _droptable 1))
  (bind _output_2 (`|GetArrayItem` _droptable 4))
  (bind _output_3 (`|GetArrayItem` _droptable))
  (bind _output_4 (`|GetArrayItem` _droptable 3))
  (bind _returnvalue (+ (`KismetMathLibrary.RandomInteger` 100) 1))
  ;[1 1 1] Reward
  (`/Engine/EditorBlueprintResources/StandardMacros.Do N` (`self.Item`)
    (:`Exit`
      (if (> _returnvalue 75)
        (`/Game/BluePrints/MainPlayerController.Get Items` PlayerController (`KismetStringLibrary.Conv_NameToString` _output_3) 1)
        (bind _asbp_player_character (cast `/Game/BluePrints/Character/BP_PlayerCharacter` (`Controller.K2_GetPawn` PlayerController)))
        (`/Game/BluePrints/Character/BP_PlayerCharacter.AddDropItem` _asbp_player_character _output_3)
        (elif (> _returnvalue 55)
          (`/Game/BluePrints/MainPlayerController.Get Items` PlayerController (`KismetStringLibrary.Conv_NameToString` _output) 1)
          (bind _asbp_player_character_2 (cast `/Game/BluePrints/Character/BP_PlayerCharacter` (`Controller.K2_GetPawn` PlayerController)))
          (`/Game/BluePrints/Character/BP_PlayerCharacter.AddDropItem` _asbp_player_character_2 _output)
          (elif (> _returnvalue 35)
            (`/Game/BluePrints/MainPlayerController.Get Items` PlayerController (`KismetStringLibrary.Conv_NameToString` (`|GetArrayItem` _droptable 2)) 1)
            (bind _asbp_player_character_3 (cast `/Game/BluePrints/Character/BP_PlayerCharacter` (`Controller.K2_GetPawn` PlayerController)))
            (`/Game/BluePrints/Character/BP_PlayerCharacter.AddDropItem` _asbp_player_character_3 "None")
            (elif (> _returnvalue 15)
              (`/Game/BluePrints/MainPlayerController.Get Items` PlayerController (`KismetStringLibrary.Conv_NameToString` _output_4) 1)
              (bind _asbp_player_character_4 (cast `/Game/BluePrints/Character/BP_PlayerCharacter` (`Controller.K2_GetPawn` PlayerController)))
              (`/Game/BluePrints/Character/BP_PlayerCharacter.AddDropItem` _asbp_player_character_4 _output_4)
              (elif (> _returnvalue 12)
                (`/Game/BluePrints/MainPlayerController.Get Items` PlayerController (`KismetStringLibrary.Conv_NameToString` _output_2) 1)
                (bind _asbp_player_character_5 (cast `/Game/BluePrints/Character/BP_PlayerCharacter` (`Controller.K2_GetPawn` PlayerController)))
                (`/Game/BluePrints/Character/BP_PlayerCharacter.AddDropItem` _asbp_player_character_5 _output_2)))))))))

(event `Respawn`
  ;[1 1 1] Respawn
  (`self.SpawnMonster`))

(event `Attack_MC`
  (params (Monster :type "/Game/BluePrints/Monster/MonsterBP/NormalMonster/BP_PoisonScorpion Object Reference"))
  ;[1 1 1] Monster's Attack
  (`self.PlayAnimMontage` Monster "/Game/Monster/Poison_Scorpion/Anim/poison_scorpion_attack_Montage.poison_scorpion_attack_Montage" 1.0 "None"))

(event `SpawnMonster`
  ;[1 1 1] Respawn
  (`|SpawnActorFromClass` (`GameplayStatics.GetObjectClass` self) (`KismetMathLibrary.MakeTransform` (.location (`self.Init Transform`)) (.rotation (`self.Init Transform`))) "Undefined" "OverrideRootScale" null (`self.Instigator`)))

(event `Damage`
  ;[1 1 1] Apply Damage
  (`self.Damage_Server` (`|GetArrayItem` (`self.TargetPlayers`))))

(event `Damage_Server`
  (params (TargetPlayer :type "/Game/BluePrints/Character/BP_PlayerCharacter Object Reference"))
  ;[1 1 1] Apply Damage
  (`GameplayStatics.ApplyDamage` TargetPlayer 10.0))

(fn `UserConstructionScript`
  (bind _droptable (`self.DropTable`))
  (`parent.UserConstructionScript`)
  (set `self.MonsterCode` "mo00005")
  (`KismetArrayLibrary.Array_Add` _droptable "et00010")
  (`KismetArrayLibrary.Array_Add` _droptable "et00018")
  (`KismetArrayLibrary.Array_Add` _droptable "et00025")
  (`KismetArrayLibrary.Array_Add` _droptable "eq40001")
  (`KismetArrayLibrary.Array_Add` _droptable "et00025"))
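; Warrior Lizard monster Blueprint that specializes a parent monster with its own health, attack and death behavior.
; It binds to parent dispatchers on BeginPlay, routing attacks through server and multicast-named events that play the attack montage.
; A separate Damage event applies damage to the first target player through a server event.
; Death plays a dying animation and binds respawn, which spawns a new instance at the initial transform.
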(event `C_Get_Socket`
  ;[1 1 1] Unused
  (set `self.EyeLocation` (`SceneComponent.GetSocketLocation` (`self.Mesh`) "Eyesight")))

(event `self.ReceiveBeginPlay`
  (`parent.ReceiveBeginPlay`)
  (add `self.Attack_Child` (delegate `C_Attack`))
  (add `self.Dead_Motion ` (delegate `Death`)))

(event `C_Attack`
  ;[1 1 1] Attack
  (`self.Attack_Server` self))

(event `Death`
  ;[1 1 1] Dead Animation
  (`SkeletalMeshComponent.PlayAnimation` (`self.Mesh`) "/Game/Monster/Warrior_Lizard/Anim/warior_lizard_dying.warior_lizard_dying" false)
  (add `self.RespawnMonster` (delegate `Resapwn`)))

(event `Attack_Server`
  (params (Monster :type "/Game/BluePrints/Monster/MonsterBP/NormalMonster/BP_WarriorLizard Object Reference"))
  ;[1 1 1] Attack
  (`self.Attack_MC` Monster))

(event `Resapwn`
  ;[1 1 1] Respawn
  (`self.SpawnMonster`))

(event `Attack_MC`
  (params (Monster :type "/Game/BluePrints/Monster/MonsterBP/NormalMonster/BP_WarriorLizard Object Reference"))
  ;[1 1 1] Attack
  (`self.PlayAnimMontage` Monster "/Game/Monster/Warrior_Lizard/Anim/warior_lizard_attack_Montage.warior_lizard_attack_Montage" 1.0 "None"))

(event `SpawnMonster`
  ;[1 1 1] Respawn
  (`|SpawnActorFromClass` (`GameplayStatics.GetObjectClass` self) (`KismetMathLibrary.MakeTransform` (.location (`self.Init Transform`)) (.rotation (`self.Init Transform`))) "Undefined" "OverrideRootScale" null (`self.Instigator`)))

(event `Damage`
  ;[1 1 1] Apply Damage
  (`self.Damage_Server` (`|GetArrayItem` (`self.TargetPlayers`))))

(event `Damage_Server`
  (params (TargetPlayer :type "/Game/BluePrints/Character/BP_PlayerCharacter Object Reference"))
  ;[1 1 1] Apply Damage
  (`GameplayStatics.ApplyDamage` TargetPlayer 10.0))

(fn `UserConstructionScript`
  (`parent.UserConstructionScript`)
  (set `self.HP` 20.0))
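; BP_Warrior_Toad is a normal monster that sets its monster code and item drop table on construction.
; On BeginPlay it binds parent dispatchers for attack, death and reward, routing the attack montage through server and multicast events.
; Death plays the dying animation and binds respawn, which spawns a new copy at the initial transform.
; Damage hits the first target player via a server event, and rewards use cascading random rolls behind a DoN.
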(event `C_Get_Socket`
  ;[1 1 1] Unsused
  (set `self.EyeLocation` (`SceneComponent.GetSocketLocation` (`self.Mesh`) "Eyesight")))

(event `self.ReceiveBeginPlay`
  (`parent.ReceiveBeginPlay`)
  (add `self.Attack_Child` (delegate `C_Attack`))
  (add `self.Dead_Motion ` (delegate `Death`))
  (add `self.Reward` (delegate `give reward`)))

(event `give reward` :!signature `self.Reward`
  (params (PlayerController :type "/Game/BluePrints/MainPlayerController Object Reference"))
  (bind _droptable (`self.DropTable`))
  (bind _returnvalue (+ (`KismetMathLibrary.RandomInteger` 100) 1))
  ;[1 1 1] Reward
  (`/Engine/EditorBlueprintResources/StandardMacros.Do N` (`self.Item`)
    (:`Exit`
      (if (> _returnvalue 84)
        (`/Game/BluePrints/MainPlayerController.Get Items` PlayerController (`KismetStringLibrary.Conv_NameToString` (`|GetArrayItem` _droptable)) 1)
        (elif (> _returnvalue 60)
          (`/Game/BluePrints/MainPlayerController.Get Items` PlayerController (`KismetStringLibrary.Conv_NameToString` (`|GetArrayItem` _droptable 1)) 1)
          (elif (> _returnvalue 44)
            (`/Game/BluePrints/MainPlayerController.Get Items` PlayerController (`KismetStringLibrary.Conv_NameToString` (`|GetArrayItem` _droptable 2)) 1)
            (elif (> _returnvalue 28)
              (`/Game/BluePrints/MainPlayerController.Get Items` PlayerController (`KismetStringLibrary.Conv_NameToString` (`|GetArrayItem` _droptable 3)) 1)
              (elif (> _returnvalue 18)
                (`/Game/BluePrints/MainPlayerController.Get Items` PlayerController (`KismetStringLibrary.Conv_NameToString` (`|GetArrayItem` _droptable 4)) 1)
                (elif (> _returnvalue 8)
                  (`/Game/BluePrints/MainPlayerController.Get Items` PlayerController (`KismetStringLibrary.Conv_NameToString` (`|GetArrayItem` _droptable 5)) 1)
                  (elif (> _returnvalue 5)
                    (`/Game/BluePrints/MainPlayerController.Get Items` PlayerController (`KismetStringLibrary.Conv_NameToString` (`|GetArrayItem` _droptable 6)) 1)))))))))))

(event `Death`
  ;[1 1 1] Death Animation
  (`SkeletalMeshComponent.PlayAnimation` (`self.Mesh`) "/Game/Monster/Warrior_Toad/Anim/warrior_toad_dying.warrior_toad_dying" false)
  (add `self.RespawnMonster` (delegate `Respawn`)))

(event `C_Attack`
  ;[1 1 1] Attack
  (`self.Attack_Server` self))

(event `Attack_Server`
  (params (Monster :type "/Game/BluePrints/Monster/MonsterBP/NormalMonster/BP_Warrior_Toad Object Reference"))
  ;[1 1 1] Attack
  (`self.Attack_MC` Monster))

(event `Respawn`
  ;[1 1 1] Respawn
  (`self.SpawnMonster`))

(event `Attack_MC`
  (params (Monster :type "/Game/BluePrints/Monster/MonsterBP/NormalMonster/BP_Warrior_Toad Object Reference"))
  ;[1 1 1] Attack
  (`self.PlayAnimMontage` Monster "/Game/Monster/Warrior_Toad/Anim/warrior_toad_attack_Montage.warrior_toad_attack_Montage" 1.0 "None"))

(event `SpawnMonster`
  ;[1 1 1] Respawn
  (`|SpawnActorFromClass` (`GameplayStatics.GetObjectClass` self) (`KismetMathLibrary.MakeTransform` (.location (`self.Init Transform`)) (.rotation (`self.Init Transform`))) "Undefined" "OverrideRootScale" null (`self.Instigator`)))

(event `Damage`
  ;[1 1 1] Apply Damage
  (`self.Damage_Server` (`|GetArrayItem` (`self.TargetPlayers`))))

(event `Damage_Server`
  (params (TargetPlayer :type "/Game/BluePrints/Character/BP_PlayerCharacter Object Reference"))
  ;[1 1 1] Apply Damage
  (`GameplayStatics.ApplyDamage` TargetPlayer 10.0))

(fn `UserConstructionScript`
  (bind _droptable (`self.DropTable`))
  (`parent.UserConstructionScript`)
  (set `self.MonsterCode` "mo00008")
  (`KismetArrayLibrary.Array_Add` _droptable "et00003")
  (`KismetArrayLibrary.Array_Add` _droptable "et00019")
  (`KismetArrayLibrary.Array_Add` _droptable "et00015")
  (`KismetArrayLibrary.Array_Add` _droptable "et00023")
  (`KismetArrayLibrary.Array_Add` _droptable "eq60001")
  (`KismetArrayLibrary.Array_Add` _droptable "eq70001")
  (`KismetArrayLibrary.Array_Add` _droptable "et00026"))
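; BP_PoweredScorpion is a child monster Blueprint for a powered scorpion with 20 HP and a 10-damage attack.
; It binds to the parent's attack dispatcher and relays the attack montage through server and multicast events, while a server event damages the first target player.
; Any hit lowers HP and turns off CanBeDamaged, with no reset here.
; At zero HP it plays the dying animation, disables capsule collision and unpossesses its AI controller.
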(event `self.ReceiveAnyDamage`
  (params (Damage :type "Float (single-precision)") (DamageType :type "DamageType Object Reference") (InstigatedBy :type "Controller Object Reference") (DamageCauser :type "Actor Object Reference"))
  (bind _output_get (set `self.HP` (- (`self.HP`) Damage)))
  (set `self.bCanBeDamaged` false)
  (if (<= _output_get 0.0)
    (`self.Death`)
    (`PrimitiveComponent.SetCollisionEnabled` (`self.CapsuleComponent`) "NoCollision")
    (`Controller.UnPossess` (`AIBlueprintHelperLibrary.GetAIController` self))))

(event `Death`
  (`SkeletalMeshComponent.PlayAnimation` (`self.Mesh`) "/Game/Monster/Powered_Scorpion/Anim/powered_scorpion_dying.powered_scorpion_dying" false))

(event `self.ReceiveBeginPlay`
  (`parent.ReceiveBeginPlay`)
  (add `self.Attack_Child` (delegate `C_Attack`)))

(event `C_Attack`
  (`self.Attack_Server` self))

(event `Attack_Server`
  (params (Monster :type "/Game/BluePrints/Monster/MonsterBP/BP_PoweredScorpion Object Reference"))
  (`self.Attack_MC` Monster))

(event `Attack_MC`
  (params (Monster :type "/Game/BluePrints/Monster/MonsterBP/BP_PoweredScorpion Object Reference"))
  (`self.PlayAnimMontage` Monster "/Game/Monster/Powered_Scorpion/Anim/powered_scorpion_attack_Montage.powered_scorpion_attack_Montage" 1.0 "None"))

(event `Damage`
  (`self.Damage_Server` (`|GetArrayItem` (`self.TargetPlayer`))))

(event `Damage_Server`
  (params (TargetPlayer :type "/Game/BluePrints/Character/BP_PlayerCharacter Object Reference"))
  (`GameplayStatics.ApplyDamage` TargetPlayer 10.0))

(fn `UserConstructionScript`
  (`parent.UserConstructionScript`)
  (set `self.HP` 20.0))
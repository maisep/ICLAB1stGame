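; Monster Blueprint that keeps track of players in range and forwards attack requests, apparently as a base for child monsters.
; SearchRange overlap events add or remove BP_PlayerCharacter entries in TargetPlayer, counting only capsule overlaps and keeping TPArraySize in step.
; The Attack event only calls CallAttackChild, so the attack behavior itself lives outside this graph.
; BeginPlay, Tick and the construction script are empty.
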(event `self.ReceiveBeginPlay`)

(event `self.ReceiveTick`
  (params (DeltaSeconds :type "Float (single-precision)")))

(event `self.SearchRange.OnComponentBeginOverlap`
  (params (OverlappedComponent :type "PrimitiveComponent Object Reference") (OtherActor :type "Actor Object Reference") (OtherComp :type "PrimitiveComponent Object Reference") (OtherBodyIndex :type Integer) (bFromSweep :type Boolean) (SweepResult :type "HitResult Structure (by ref)"))
  (bind _targetplayer (`self.TargetPlayer`))
  (bind _asbp_player_character (cast `/Game/BluePrints/Character/BP_PlayerCharacter` OtherActor))
  (if (== (`Character.CapsuleComponent` _asbp_player_character) OtherComp)
    (if (== (`KismetArrayLibrary.Array_Find` _targetplayer _asbp_player_character) -1)
      (`KismetArrayLibrary.Array_Add` _targetplayer _asbp_player_character)
      (`/Engine/EditorBlueprintResources/StandardMacros.IncrementInt` (`self.TPArraySize`)))))

(event `self.SearchRange.OnComponentEndOverlap`
  (params (OverlappedComponent :type "PrimitiveComponent Object Reference") (OtherActor :type "Actor Object Reference") (OtherComp :type "PrimitiveComponent Object Reference") (OtherBodyIndex :type Integer))
  (bind _targetplayer (`self.TargetPlayer`))
  (bind _asbp_player_character (cast `/Game/BluePrints/Character/BP_PlayerCharacter` OtherActor))
  (if (== (`Character.CapsuleComponent` _asbp_player_character) OtherComp)
    (`KismetArrayLibrary.Array_Remove` _targetplayer (`KismetArrayLibrary.Array_Find` _targetplayer _asbp_player_character))
    (`/Engine/EditorBlueprintResources/StandardMacros.DecrementInt` (`self.TPArraySize`))))

(event `Attack`
  (`self.Attack_Child`))

(fn `UserConstructionScript`)
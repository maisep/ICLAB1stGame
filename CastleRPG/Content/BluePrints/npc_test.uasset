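; Test NPC Blueprint that offers buyable equipment and usable item lists to a player standing near it.
; On BeginPlay it applies its material to the cube mesh.
; When a ThirdPersonCharacter enters the box, it copies its UI list and item lists into that character's MainPlayerController and sets UiCheck.
; Leaving the box clears only UiCheck, so the copied lists stay on the controller.
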(event `self.ReceiveBeginPlay`
  (`PrimitiveComponent.SetMaterial` (`self.Cube`) 0 (`self.mat`)))

(event `self.Box.OnComponentBeginOverlap`
  (params (OverlappedComponent :type "PrimitiveComponent Object Reference") (OtherActor :type "Actor Object Reference") (OtherComp :type "PrimitiveComponent Object Reference") (OtherBodyIndex :type Integer) (bFromSweep :type Boolean) (SweepResult :type "HitResult Structure (by ref)"))
  (bind _asthird_person_character (cast `/Game/PN_MeadowFlowers/UE4ThirdPersonTemplate/ThirdPersonBP/Blueprints/ThirdPersonCharacter` OtherActor))
  (bind _asmain_player_controller (cast `/Game/BluePrints/modes/MainPlayerController` (`Pawn.GetController` _asthird_person_character)))
  (set `/Game/BluePrints/modes/MainPlayerController.ui_list` (`self.Ui List`) _asmain_player_controller)
  (set `/Game/BluePrints/modes/MainPlayerController.ui_check` true _asmain_player_controller)
  (set `/Game/BluePrints/modes/MainPlayerController.eq_buy_items_a` (`self.eq_items_a`) _asmain_player_controller)
  (set `/Game/BluePrints/modes/MainPlayerController.eq_buy_items_w` (`self.eq_items_w`) _asmain_player_controller)
  (set `/Game/BluePrints/modes/MainPlayerController.us_buy_items` (`self.us_items`) _asmain_player_controller))

(event `self.Box.OnComponentEndOverlap`
  (params (OverlappedComponent :type "PrimitiveComponent Object Reference") (OtherActor :type "Actor Object Reference") (OtherComp :type "PrimitiveComponent Object Reference") (OtherBodyIndex :type Integer))
  (bind _asthird_person_character (cast `/Game/PN_MeadowFlowers/UE4ThirdPersonTemplate/ThirdPersonBP/Blueprints/ThirdPersonCharacter` OtherActor))
  (bind _asmain_player_controller (cast `/Game/BluePrints/modes/MainPlayerController` (`Pawn.GetController` _asthird_person_character)))
  (set `/Game/BluePrints/modes/MainPlayerController.ui_check` false _asmain_player_controller))

(event `self.ReceiveTick`
  (params (DeltaSeconds :type "Float (single-precision)")))

(fn `UserConstructionScript`)
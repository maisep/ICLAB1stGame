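; Game mode blueprint that relays chat messages and the player list to player controllers.
; UpdatePlayerlist copies PlayerList to every MainPlayerController.
; The ChatMSG RepNotify appends to ChatLog, then finds each BP_PlayerCharacter's MainPlayerController to add the message to its game instance log and print it.
; The PlayerList and Nick_memo RepNotifies, BeginPlay and Tick are empty.
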(event `self.ReceiveBeginPlay`)

(event `UpdatePlayerlist`
  (bind _outactors (`GameplayStatics.GetAllActorsOfClass` "/Game/BluePrints/MainPlayerController.MainPlayerController_C"))
  (for _array_element _outactors
    (set `/Game/BluePrints/MainPlayerController.PlayerList` (`self.PlayerList`) _array_element)))

(fn `OnRep_ChatMSG`
  (bind _chatmsg (`self.ChatMSG`))
  (`KismetArrayLibrary.Array_Add` (`self.ChatLog`) (`self.ChatMSG`))
  (bind _outactors (`GameplayStatics.GetAllActorsOfClass` "/Game/BluePrints/Character/BP_PlayerCharacter.BP_PlayerCharacter_C"))
  (for _array_element _outactors
    (bind _asmain_player_controller (cast `/Game/BluePrints/MainPlayerController` (`Pawn.GetController` _array_element)))
    (`KismetArrayLibrary.Array_Add` (`/Game/BluePrints/main_instance.ChatLog` (`/Game/BluePrints/MainPlayerController.As Main Instance` _asmain_player_controller)) _chatmsg)
    (`/Game/BluePrints/MainPlayerController.PrintChat` _asmain_player_controller _chatmsg)))

(fn `OnRep_Nick_memo`)

(fn `OnRep_PlayerList`)

(fn `UserConstructionScript`)